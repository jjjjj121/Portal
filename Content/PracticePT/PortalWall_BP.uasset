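; Portal-placeable wall actor that spawns or moves the single blue or red portal at a hit point, scaling its mesh from width and height.
; SpawnPortal converts the hit to wall-local space, nudges it off the surface, and clamps both Y and Z using SizeWidth.
; Per-axis distance tests reject placement overlapping the other portal.
; Successful placement plays a sound and, when the other portal exists, sets link flags.
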(event `self.ReceiveBeginPlay`)

(fn `Check Portal`
  (params (`Hit Point Y` :type "Float (double-precision)") (`Hit Point Z` :type "Float (double-precision)") (`Portal Radius Y` :type "Float (double-precision)") (`Portal Radius Z` :type "Float (double-precision)"))
  (returns (`New Y` :type "Float (double-precision)") (`New Z` :type "Float (double-precision)"))
  (locals (`New Location Y` :type "Float (double-precision)" :default 0.0) (`New Location Z` :type "Float (double-precision)" :default 0.0) (TestY :type "Float (double-precision)" :default 250.0) (`Test Z` :type "Float (double-precision)"))
  ;[1 1 1] Y좌표 조정
  (bind _newlocation (`self.Mediate Portal` (`local.Hit Point Y`) (`local.Portal Radius Y`)))
  (set `local.New Location Y` _newlocation)
  ;[1 1 1] Z좌표 조정
  (bind _newlocation_2 (`self.Mediate Portal` (`local.Hit Point Z`) (`local.Portal Radius Z`)))
  (set `local.New Location Z` _newlocation_2)
  (return (`local.New Location Y`) (`local.New Location Z`)))

(fn `Check X Portal`
  (params (`A Location X` :type "Float (double-precision)") (`B Location Y` :type "Float (double-precision)"))
  (returns (`Overlap?` :type Boolean))
  (if (< (`KismetMathLibrary.Abs` (- (`local.A Location X`) (`local.B Location Y`))) 1.0)
    (return true)
    (else
      (return false))))

(fn `CheckPortalPlace`
  (params (APortalLocation :type "Float (double-precision)") (BPortalLocation :type "Float (double-precision)") (`Portal Size` :type "Float (double-precision)"))
  (returns (PortalOverlap :type Boolean))
  (if (< (`KismetMathLibrary.Abs` (- (`local.APortalLocation`) (`local.BPortalLocation`))) (`local.Portal Size`))
    (return true)
    (else
      (return false))))

(fn `IsPortalOverlap`
  (params (`Location A` :type "Vector Structure") (`Location B` :type "Vector Structure") (`Portal Y size` :type "Float (double-precision)") (`Portal Z size` :type "Float (double-precision)"))
  (returns (PortalOverlap :type Boolean))
  (locals (OverlapY :type Boolean :default false) (OverlapZ :type Boolean :default false) (OverlapX :type Boolean :default false))
  (bind (_location_a_x _location_a_y _location_a_z) (`KismetMathLibrary.BreakVector` (`local.Location A`)))
  (bind (_location_b_x _location_b_y _location_b_z) (`KismetMathLibrary.BreakVector` (`local.Location B`)))
  (bind (_location_a_x_2 _location_a_y_2) (`KismetMathLibrary.BreakVector` (`local.Location A`)))
  (bind (_location_b_x_2 _location_b_y_2) (`KismetMathLibrary.BreakVector` (`local.Location B`)))
  (bind _location_a_x_3 (`KismetMathLibrary.BreakVector` (`local.Location A`)))
  (bind _location_b_x_3 (`KismetMathLibrary.BreakVector` (`local.Location B`)))
  ;[1 1 1] y좌표 검사
  (bind _portaloverlap (`self.CheckPortalPlace` _location_a_y_2 _location_b_y_2 (`local.Portal Y size`)))
  (set `local.OverlapY` _portaloverlap)
  ;[1 1 1] z좌표 검사
  (bind _portaloverlap_2 (`self.CheckPortalPlace` _location_a_z _location_b_z (`local.Portal Z size`)))
  (set `local.OverlapZ` _portaloverlap_2)
  (bind _overlap_ (`self.Check X Portal` _location_a_x_3 _location_b_x_3))
  (set `local.OverlapX` _overlap_)
  (if (and (`local.OverlapY`) (`local.OverlapZ`) (`local.OverlapX`))
    (return true)
    (else
      (return false))))

(fn `Mediate Portal`
  (params (location :type "Float (double-precision)") (PortalRadius :type "Float (double-precision)"))
  (returns (NewLocation :type "Float (double-precision)"))
  (locals (Amount :type "Float (double-precision)"))
  (bind _returnvalue (- (- (/ (`self.SizeWidth`) 2.0) (`local.PortalRadius`)) (`KismetMathLibrary.Abs` (`local.location`))))
  ;[1 1 1] Y 또는 Z좌표 조정
  ;;[1 1 1] 음수면 실행(범위를 벗어나야 음수)
  (if (< _returnvalue 0.0)
    ;;[1 1 1] 좌표 양 저장
    (set `local.Amount` _returnvalue)
    ;;[1 1 1] New 좌표 저장
    (set `local.Amount` (+ (`local.Amount`) (`KismetMathLibrary.Abs` (`local.location`))))
    (if (> (`local.location`) 0.0)
      ;;[1 1 1] location이 양수라면
      (return (`local.Amount`))
      (else
        ;;[1 1 1] location이 음수라면
        (return (- 0.0 (`local.Amount`)))))
    (else
      ;;[1 1 1] false 시 기존값 그대로 반환
      (return (`local.location`)))))

(fn `Spawn Portal`
  (params (`Is Portal A` :type Boolean) (`Hit Point` :type "Vector Structure"))
  (locals (PortalY :type "Float (double-precision)" :default 249.0) (PortalZ :type "Float (double-precision)" :default 275.0) (`Local Point vector` :type "Vector Structure"))
  (bind _returnvalue (`self.K2_GetActorRotation`))
  (bind _returnvalue_2 (`self.K2_GetActorRotation`))
  (bind _returnvalue_3 (`KismetMathLibrary.TransformLocation` (`self.GetTransform`) (`local.Local Point vector`)))
  (bind _returnvalue_4 (`KismetMathLibrary.TransformLocation` (`self.GetTransform`) (`local.Local Point vector`)))
  (bind _output_get (set `local.Local Point vector` (`KismetMathLibrary.InverseTransformLocation` (`self.GetTransform`) (`local.Hit Point`))))
  (bind (_new_y _new_z) (`self.Check Portal` (.y _output_get) (.z _output_get) (/ (`local.PortalY`) 2.0) (/ (`local.PortalZ`) 2.0)))
  ;[1 1 1] 조정된 위치 좌표 vector
  (set `local.Local Point vector` (`KismetMathLibrary.MakeVector` (+ (.x _output_get) 0.01) _new_y _new_z))
  (if (`local.Is Portal A`)
    ;[1 1 1] APortal 생성
    ;;[1 1 1] A포탈 존재?
    (bind _returnvalue_5 (`GameplayStatics.GetActorOfClass` "/Game/PracticePT/Portal_Blue.Portal_Blue_C"))
    (`/Engine/EditorBlueprintResources/StandardMacros.IsValid` _returnvalue_5
      (:`Is Valid`
        ;;[1 1 1] B포탈 존재?
        (bind _returnvalue_6 (`GameplayStatics.GetActorOfClass` "/Game/PracticePT/Portal_Red.Portal_Red_C"))
        (`/Engine/EditorBlueprintResources/StandardMacros.IsValid` _returnvalue_6
          (:`Is Valid`
            ;;[1 1 1] B포탈이 존재하므로 A포탈을 생성하려는 경우 오버랩 유무 체크
            (bind _portaloverlap (`self.IsPortalOverlap` (`local.Local Point vector`) (`KismetMathLibrary.InverseTransformLocation` (`self.GetTransform`) (`self.K2_GetActorLocation` _returnvalue_6)) (`local.PortalY`) (`local.PortalZ`)))
            (if (not _portaloverlap)
              (set `/Game/PracticePT/Portal_Red.Is Link?` true _returnvalue_6)
              (`SceneComponent.K2_SetRelativeLocationAndRotation` (`/Game/PracticePT/Portal_Blue.DefaultSceneRoot` _returnvalue_5) _returnvalue_3 _returnvalue false false :!label _label)
              (`GameplayStatics.PlaySound2D` "/Engine/VREditor/Sounds/UI/Teleport_Mode_Entered.Teleport_Mode_Entered" 1.0 1.0 0.0 null null :!label _label_2)))
          (:`Is Not Valid`
            (goto _label))))
      (:`Is Not Valid`
        (bind _returnvalue_7 (`GameplayStatics.GetActorOfClass` "/Game/PracticePT/Portal_Red.Portal_Red_C"))
        (`/Engine/EditorBlueprintResources/StandardMacros.IsValid` _returnvalue_7
          (:`Is Valid`
            ;;[1 1 1] B포탈이 존재하므로 A포탈을 생성하려는 경우 오버랩 유무 체크
            (bind _portaloverlap_2 (`self.IsPortalOverlap` (`local.Local Point vector`) (`KismetMathLibrary.InverseTransformLocation` (`self.GetTransform`) (`self.K2_GetActorLocation` _returnvalue_7)) (`local.PortalY`) (`local.PortalZ`)))
            (if (not _portaloverlap_2)
              (set `/Game/PracticePT/Portal_Red.Is Link?` true _returnvalue_7)
              (`|SpawnActorFromClass` "/Game/PracticePT/Portal_Blue.Portal_Blue_C" (`KismetMathLibrary.MakeTransform` _returnvalue_3 _returnvalue) "Undefined" "OverrideRootScale" null true null) ; Link 체크
              (goto _label_2)))
          (:`Is Not Valid`
            (`|SpawnActorFromClass` "/Game/PracticePT/Portal_Blue.Portal_Blue_C" (`KismetMathLibrary.MakeTransform` _returnvalue_3 _returnvalue) "Undefined" "OverrideRootScale" null false null) ; Link 체크 해제
            (goto _label_2)))))
    (else
      ;[1 1 1] BPortal 생성
      ;;[1 1 1] B포탈 존재?
      (bind _returnvalue_8 (`GameplayStatics.GetActorOfClass` "/Game/PracticePT/Portal_Red.Portal_Red_C"))
      (`/Engine/EditorBlueprintResources/StandardMacros.IsValid` _returnvalue_8
        (:`Is Valid`
          ;;[1 1 1] A포탈 존재?
          (bind _returnvalue_9 (`GameplayStatics.GetActorOfClass` "/Game/PracticePT/Portal_Blue.Portal_Blue_C"))
          (`/Engine/EditorBlueprintResources/StandardMacros.IsValid` _returnvalue_9
            (:`Is Valid`
              ;;[1 1 1] B포탈이 존재하므로 A포탈을 생성하려는 경우 오버랩 유무 체크
              (bind _portaloverlap_3 (`self.IsPortalOverlap` (`KismetMathLibrary.InverseTransformLocation` (`self.GetTransform`) (`self.K2_GetActorLocation` _returnvalue_9)) (`local.Local Point vector`) (`local.PortalY`) (`local.PortalZ`)))
              (if (not _portaloverlap_3)
                (set `/Game/PracticePT/Portal_Blue.Is Link?` true _returnvalue_9)
                (`SceneComponent.K2_SetRelativeLocationAndRotation` (`Actor.RootComponent` _returnvalue_8) _returnvalue_4 _returnvalue_2 false false :!label _label_3)
                (`GameplayStatics.PlaySound2D` "/Engine/VREditor/Sounds/UI/Teleport_Mode_Entered.Teleport_Mode_Entered" 1.0 1.0 0.0 null null :!label _label_4)))
            (:`Is Not Valid`
              (goto _label_3))))
        (:`Is Not Valid`
          (bind _returnvalue_10 (`GameplayStatics.GetActorOfClass` "/Game/PracticePT/Portal_Blue.Portal_Blue_C"))
          (`/Engine/EditorBlueprintResources/StandardMacros.IsValid` _returnvalue_10
            (:`Is Valid`
              ;;[1 1 1] B포탈이 존재하므로 A포탈을 생성하려는 경우 오버랩 유무 체크
              (bind _portaloverlap_4 (`self.IsPortalOverlap` (`KismetMathLibrary.InverseTransformLocation` (`self.GetTransform`) (`self.K2_GetActorLocation` _returnvalue_10)) (`local.Local Point vector`) (`local.PortalY`) (`local.PortalZ`)))
              (if (not _portaloverlap_4)
                (set `/Game/PracticePT/Portal_Blue.Is Link?` true _returnvalue_10)
                (`|SpawnActorFromClass` "/Game/PracticePT/Portal_Red.Portal_Red_C" (`KismetMathLibrary.MakeTransform` _returnvalue_4 _returnvalue_2) "Undefined" "OverrideRootScale" null true null)
                (goto _label_4)))
            (:`Is Not Valid`
              (`|SpawnActorFromClass` "/Game/PracticePT/Portal_Red.Portal_Red_C" (`KismetMathLibrary.MakeTransform` _returnvalue_4 _returnvalue_2) "Undefined" "OverrideRootScale" null false null)
              (goto _label_4))))))))

(fn `UserConstructionScript`
  (`SceneComponent.SetWorldScale3D` (`self.Wall`) (`KismetMathLibrary.MakeVector` 1.0 (/ (`self.SizeWidth`) 100.0) (/ (`self.SizeHeight`) 100.0))))